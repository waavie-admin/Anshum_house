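; Desktop HUD Blueprint for an architectural visualization player that creates the main widget and acts as its bridge for menus, minimap, tips, floor info and light messages.
; Input events for toggling, selecting, moving and going back forward to the widget, while menu toggles also switch the cursor through the desktop player controller.
; It tracks options-menu state, answers edit and decal mode queries, and animates the crosshair with a reversible timeline.
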(event Custom|OnToggleMainMenu
  (bind _mainwidget (Variables|Default|GetMainWidget))
  (bind _mainmenu_btn (Variables|/Game/ArchVis/Blueprint/UMG/MainWidget_BP.MainWidget_BP_C|GetMainMenu_BTN _mainwidget))
  ;[1 1 1] Toggle main menu
  (Default|OnClicked _mainmenu_btn)
  (CallFunction|ToggleCursor (Default|GetEnabeld _mainmenu_btn)))

(event Custom|ToggleOptionsMenu
  ;[1 1 1] Toggle option open and close
  (bind _newenable (Default|OnToggleOptionMenu (Variables|Default|GetMainWidget) (not (Variables|Options|GetbIsMenuOpen))))
  (bind _output_get (Variables|Options|SetbIsMenuOpen _newenable))
  (CallFunction|ToggleCursor _output_get))

(event Custom|CloseOptionsButton
  ;[1 1 1] Toggle option open and close
  (bind _newenable (Default|OnToggleOptionMenu (Variables|Default|GetMainWidget) (not (Variables|Options|GetbIsMenuOpen))))
  (bind _output_get (Variables|Options|SetbIsMenuOpen _newenable))
  (CallFunction|ToggleCursor _output_get))

(event Custom|OnHorizontalMove
  (params (bNewMove :type Boolean) (bLeft :type Boolean))
  ;[1 1 1] Move in menus using keyboard or controller buttons
  (Default|OnHorizontalMove (Variables|Default|GetMainWidget) bNewMove bLeft))

(event Custom|OnSelectOption
  ;[1 1 1] Select options using keyboard or controller button
  (Default|OnSelectOption (Variables|Default|GetMainWidget)))

(event Custom|AnimateCrosshair
  (params (bNewFocus :type Boolean))
  ;[1 1 1] Animate crosshair
  (if bNewFocus
    (bind _radius (Timeline|FocusAnimation PlayFromStart)
      (:Update
        (Default|AnimateCrosshair (Variables|Default|GetMainWidget) _radius)))
    (else
      (Timeline|FocusAnimation ReverseFromEnd))))

(event Custom|OnToggleMinimap
  ;[1 1 1] Toggle Minimap
  (Default|OnClicked (Variables|/Game/ArchVis/Blueprint/UMG/MainWidget_BP.MainWidget_BP_C|GetMinimap_BTN (Variables|Default|GetMainWidget))))

(event Custom|OnVerticalMove
  (params (bNewMove :type Boolean) (bDown :type Boolean))
  ;[1 1 1] Move in menus using keyboard or controller buttons
  (Default|OnVerticalMove (Variables|Default|GetMainWidget) bNewMove bDown))

(event Custom|OnBackButton
  ;[1 1 1] Back called from controller
  (Default|OnBackButton (Variables|Default|GetMainWidget)))

(event EventBeginPlay
  ;[1 1 1] Create the main widget and add to screen
  (bind _returnvalue (UserInterface|CreateWidget "/Game/ArchVis/Blueprint/UMG/MainWidget_BP.MainWidget_BP_C" (Game|Player|GetOwningPlayerController)))
  (bind _output_get (Variables|Default|SetMainWidget _returnvalue))
  (UserInterface|Viewport|AddtoViewport _output_get 0)
  ;[1 1 1] Bind close option menu button
  (EventDispatchers|BindEventtoCloseOptionsMenu (Variables|Default|GetMainWidget) (EventDispatchers|CreateEvent :!event Custom|CloseOptionsButton)))

(fn ConstructionScript)

(fn ToggleCursor
  (params (bNewEnable :type Boolean))
  ;[1 1 1] Call toggle mouse cursor from player controller class
  (bind _asdesktop_player_controller_bp (Utilities|Casting|CastToDesktopPlayerController_BP (Game|Player|GetOwningPlayerController)))
  (Default|ToggleCursor _asdesktop_player_controller_bp bNewEnable))

(fn CheckIsMenuOpen
  (return (Variables|Options|GetbIsMenuOpen)))

(fn IsinEditMode
  (if (Variables|Options|GetbIsMenuOpen)
    (if (Utilities|Enum|Equal(Enum) (Variables|/Game/ArchVis/Blueprint/UMG/MainWidget_BP.MainWidget_BP_C|GetCurrentMenu (Variables|Default|GetMainWidget)) "NewEnumerator4")
      (return (Default|IsinEditMode (Variables|/Game/ArchVis/Blueprint/UMG/MainWidget_BP.MainWidget_BP_C|GetMainOptions_BP (Variables|Default|GetMainWidget))))
      (else
        _)))
  (return false))

(fn IsinDecalMode
  (if (Utilities|Enum|Equal(Enum) (Variables|/Game/ArchVis/Blueprint/UMG/MainWidget_BP.MainWidget_BP_C|GetCurrentMenu (Variables|Default|GetMainWidget)) "NewEnumerator4")
    (return (Default|IsinDecalMode (Variables|/Game/ArchVis/Blueprint/UMG/MainWidget_BP.MainWidget_BP_C|GetMainOptions_BP (Variables|Default|GetMainWidget))))
    (else
      (return false))))

(fn ToggleTipMode
  (params (bNewController :type Boolean))
  ;[1 1 1] Toggle tip mode on main widget
  (Default|ToggleTipMode (Variables|Default|GetMainWidget) bNewController))

(fn UpdateFloorInfo
  (params (NewFloor :type Floor%20Info%20BP%20Object%20Reference))
  (bind _mainwidget (Variables|Default|GetMainWidget))
  ;[1 1 1] Call update floor info from main widget
  (Utilities|IsValid _mainwidget
    (:Is%20Valid
      (Default|UpdateFloorInfo _mainwidget NewFloor))))

(fn ToggleLightMessage
  (params (bNewShow :type Boolean))
  (Utilities|IsValid (Variables|Default|GetMainWidget)
    (:Is%20Valid
      (Default|ToggleLightMessage (Variables|Default|GetMainWidget) bNewShow))))