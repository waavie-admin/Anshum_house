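; Save data Blueprint for the ArchVis project that stores named profiles and the per-actor data belonging to each.
; AddProfile registers a unique name and appends actor data, or with override replaces the entry matching both profile and actor.
; Other functions check whether a profile exists, gather its entries, or delete it by walking the data array backwards so removals are safe.
; AddLight is an empty stub.
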(fn AddProfile
  (params (NewProfileName :type String) (NewActorData :type Save%20Table%20BP%20Structure) (bNewOverride :type Boolean))
  (LocalVariables|SetTempData NewActorData)
  (LocalVariables|SetTempProfileName NewProfileName)
  (Utilities|Array|AddUnique (Variables|Default|GetProfiles) (LocalVariables|GetTempProfileName))
  (if bNewOverride
    (LocalVariables|SetbFound false)
    ;[1 1 1] If we must override data then find the element and override to new data
    (bind (_array_element _array_index) (Utilities|Array|ForEachLoopwithBreak (Variables|Default|GetActorsData) :!label _label)
      (:LoopBody
        (if (and (Utilities|Enum|Equal(Enum) (.ProfileName (Utilities|Struct|BreakSaveTable_BP _array_element)) (LocalVariables|GetTempProfileName)) (== (.Actor (Utilities|Struct|BreakSaveTable_BP _array_element)) (.Actor (Utilities|Struct|BreakSaveTable_BP (LocalVariables|GetTempData)))))
          (LocalVariables|SetbFound true)
          (Utilities|Array|SetArrayElem (Variables|Default|GetActorsData) _array_index (LocalVariables|GetTempData))
          (goto _label Break)))
      (:Completed
        ;[1 1 1] If we didn't found data to override just add directly into array
        (if (not (LocalVariables|GetbFound))
          (Utilities|Array|Add (Variables|Default|GetActorsData) (LocalVariables|GetTempData)))))
    (else
      ;[1 1 1] If we don't need to override anything then just add to new data table to Actors data array
      (Utilities|Array|Add (Variables|Default|GetActorsData) (LocalVariables|GetTempData)))))

(fn IsProfileExists
  (params (NewProfileName :type String))
  ;[1 1 1] Check if profile with this name exists or not
  (return (> (Utilities|Array|FindItem (Variables|Default|GetProfiles) NewProfileName) -1)))

(fn GetProfileData
  (params (NewProfileName :type String))
  ;[1 1 1] Get data for desired profile
  (LocalVariables|SetTempProfileName NewProfileName)
  (for _array_element (Variables|Default|GetActorsData)
    (if (Utilities|Enum|Equal(Enum) (LocalVariables|GetTempProfileName) (.ProfileName (Utilities|Struct|BreakSaveTable_BP _array_element)))
      (Utilities|Array|Add (LocalVariables|GetDataTable) _array_element)))
  (return (LocalVariables|GetDataTable)))

(fn AddLight)

(fn DeleteProfile
  (params (NewProfileName :type String))
  (bind _actorsdata (Variables|Default|GetActorsData))
  ;[1 1 1] Find all data to the desired profile and remove from ActorsData
  (bind _output_get (LocalVariables|SetTempProfileName NewProfileName))
  (bind _returnvalue (Utilities|Array|RemoveItem (Variables|Default|GetProfiles) _output_get))
  (if _returnvalue
    (LocalVariables|SetCurrentIndex (- (Utilities|Array|Length (Variables|Default|GetActorsData)) 1))
    (while (> (LocalVariables|GetCurrentIndex) -1)
      (if (> (Utilities|Array|Length _actorsdata) (LocalVariables|GetCurrentIndex))
        (if (Utilities|Enum|Equal(Enum) (.ProfileName (Utilities|Struct|BreakSaveTable_BP (Utilities|Array|Get(acopy) _actorsdata (LocalVariables|GetCurrentIndex)))) (LocalVariables|GetTempProfileName))
          (Utilities|Array|RemoveIndex (Variables|Default|GetActorsData) (LocalVariables|GetCurrentIndex)))
        (LocalVariables|SetCurrentIndex (- (LocalVariables|GetCurrentIndex) 1))))))