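; FloorInfo_BP is a floor trigger actor that reports itself to the desktop player controller when a player's pawn touches its collision box.
; At BeginPlay it scans for pawns already overlapping FloorCollision, and later begin-overlap events feed the same logic.
; That logic casts to the pawn's DesktopPlayerController_BP, waits briefly, calls UpdateFloorInfo with itself and sets Initialized, which gates only the startup scan.
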(event OnComponentBeginOverlap(FloorCollision)
  (params (OverlappedComponent :type Primitive%20Component%20Object%20Reference) (OtherActor :type Actor%20Object%20Reference) (OtherComp :type Primitive%20Component%20Object%20Reference) (OtherBodyIndex :type Integer) (bFromSweep :type Boolean) (SweepResult :type Hit%20Result%20Structure%20%28by%20ref%29))
  ;[1 1 1] Update floor info after touching collision box
  (Variables|Internal|SetOverlapActor OtherActor)
  (bind _aspawn (Utilities|Casting|CastToPawn (Variables|Internal|GetOverlapActor)))
  (bind _asdesktop_player_controller_bp (Utilities|Casting|CastToDesktopPlayerController_BP (Pawn|GetController _aspawn)))
  (Utilities|FlowControl|Delay 0.5)
  (Default|UpdateFloorInfo _asdesktop_player_controller_bp self)
  (Variables|Internal|SetbInitialized true)
  (Utilities|Array|ForEachLoopwithBreak (Collision|GetOverlappingActors (Variables|Default|GetFloorCollision) "/Script/Engine.Pawn" :!class /Script/Engine.PrimitiveComponent)) ; enters at Break
)

(event EventBeginPlay
  (if (not (Variables|Internal|GetbInitialized))
    (bind _array_element (Utilities|Array|ForEachLoopwithBreak (Collision|GetOverlappingActors (Variables|Default|GetFloorCollision) "/Script/Engine.Pawn" :!class /Script/Engine.PrimitiveComponent) :!label _label)
      (:LoopBody
        (Variables|Internal|SetOverlapActor _array_element)
        ;[1 1 1] Update floor info after touching collision box
        (bind _aspawn (Utilities|Casting|CastToPawn (Variables|Internal|GetOverlapActor)))
        (bind _asdesktop_player_controller_bp (Utilities|Casting|CastToDesktopPlayerController_BP (Pawn|GetController _aspawn)))
        (Utilities|FlowControl|Delay 0.5)
        (Default|UpdateFloorInfo _asdesktop_player_controller_bp self)
        (Variables|Internal|SetbInitialized true)
        (goto _label Break)))))

(fn ConstructionScript)