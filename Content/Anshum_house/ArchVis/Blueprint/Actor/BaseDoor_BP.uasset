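; Base door actor that opens automatically when Character_BP enters its collision box and closes when it leaves.
; The DoorAlpha timeline, rate-scaled by an animation speed, lerps either mesh world rotation or relative location for rotating or sliding doors.
; Toggling always plays from start or reverses from end, so interrupted motion jumps.
; The construction script configures the trigger box and can capture the actor's transform as the closed pose.
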(event OnComponentBeginOverlap(DoorCollision)
  (params (OverlappedComponent :type Primitive%20Component%20Object%20Reference) (OtherActor :type Actor%20Object%20Reference) (OtherComp :type Primitive%20Component%20Object%20Reference) (OtherBodyIndex :type Integer) (bFromSweep :type Boolean) (SweepResult :type Hit%20Result%20Structure%20%28by%20ref%29))
  ;[1 1 1] Toggle door open or close when player has overlap with collision box
  (Utilities|Casting|CastToCharacter_BP OtherActor)
  (CallFunction|ToggleDoor true))

(event OnComponentEndOverlap(DoorCollision)
  (params (OverlappedComponent :type Primitive%20Component%20Object%20Reference) (OtherActor :type Actor%20Object%20Reference) (OtherComp :type Primitive%20Component%20Object%20Reference) (OtherBodyIndex :type Integer))
  ;[1 1 1] Toggle door open or close when player has overlap with collision box
  (Utilities|Casting|CastToCharacter_BP OtherActor)
  (CallFunction|ToggleDoor false))

(event Custom|ToggleDoor
  (params (bNewOpen :type Boolean))
  (bind _opentransform (Variables|Door|GetOpenTransform))
  (bind (_location _rotation) (Math|Transform|BreakTransform _opentransform))
  (if bNewOpen
    (bind _alpha (Timeline|DoorAlpha PlayFromStart)
      (:Update
        (switch Utilities|FlowControl|Switch|SwitchonEDoorTypes (Variables|Door|GetDoorType)
          (:NewEnumerator0
            (Transformation|SetWorldRotation (Variables|Character|GetMesh) (Math|Rotator|Lerp(Rotator) (.Rotation (Math|Transform|BreakTransform (Variables|Door|GetCloseTransform))) _rotation _alpha true) false false))
          (:NewEnumerator3
            (Transformation|SetRelativeLocation (Variables|Character|GetMesh) (Math|Vector|Lerp(Vector) "0, 0, 0" _location _alpha) false false)))))
    (else
      (Timeline|DoorAlpha ReverseFromEnd))))

(event EventBeginPlay
  (bind _dooralpha (Variables|Default|GetDoorAlpha))
  ;[1 1 1] Set play rate for door animation
  (|CallParentFunction)
  (Components|Timeline|SetPlayRate _dooralpha (* (Components|Animation|GetPlayRate _dooralpha) (Variables|Door|GetDoorAnimationSpeed))))

(fn ConstructionScript
  (bind _collisiontransform (Variables|Door|GetCollisionTransform))
  (bind (_location _rotation _scale) (Math|Transform|BreakTransform _collisiontransform))
  (|CallParentFunction)
  (Variables|Default|SetbMoveable false)
  ;[1 1 1] Update collision box
  (Transformation|AddRelativeLocation (Variables|Default|GetDoorCollision) _location false false)
  (Transformation|SetWorldRotation (Variables|Default|GetDoorCollision) _rotation false false)
  (Transformation|SetWorldScale3D (Variables|Default|GetDoorCollision) _scale)
  (Components|Box|SetBoxExtent (Variables|Default|GetDoorCollision) (Variables|Door|GetCollisionBoxExtent) true)
  ;[1 1 1] Set current actor transform as close transform
  (if (Variables|Door|GetbUseCurrentTransformForClose)
    (Variables|Door|SetCloseTransform (Transformation|GetActorTransform))))