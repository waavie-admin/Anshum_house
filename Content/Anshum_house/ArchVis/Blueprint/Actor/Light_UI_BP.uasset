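; ArchVis UI actor that links a button info setup to a referenced Light for adjusting its intensity and color.
; The construction script fixes the button and submenu types in UIInfo, then detaches and snaps the actor onto LightReference when valid.
; Intensity changes remap a normalized value into the secondary slide's desired range, color changes apply UIInfo's desired color, and OnUpdateInfo replaces the stored UIInfo.
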(fn ConstructionScript
  (bind _lightreference (Variables|Options|GetLightReference))
  (Variables|Options|SetUI_Info (Utilities|Struct|MakeFButtonInfo "NewEnumerator7" (.DisplayName (Utilities|Struct|BreakFButtonInfo (Variables|Options|GetUI_Info))) (.FontSize (Utilities|Struct|BreakFButtonInfo (Variables|Options|GetUI_Info))) (.TextSpace (Utilities|Struct|BreakFButtonInfo (Variables|Options|GetUI_Info))) (.Size (Utilities|Struct|BreakFButtonInfo (Variables|Options|GetUI_Info))) (.Normal (Utilities|Struct|BreakFButtonInfo (Variables|Options|GetUI_Info))) (.Hovered (Utilities|Struct|BreakFButtonInfo (Variables|Options|GetUI_Info))) (.Selected (Utilities|Struct|BreakFButtonInfo (Variables|Options|GetUI_Info))) (.Slide (Utilities|Struct|BreakFButtonInfo (Variables|Options|GetUI_Info))) (.Color (Utilities|Struct|BreakFButtonInfo (Variables|Options|GetUI_Info))) "NewEnumerator4" (.bSpaceToEnter (Utilities|Struct|BreakFButtonInfo (Variables|Options|GetUI_Info)))))
  (Transformation|DetachFromActor "KeepWorld" "KeepWorld" "KeepWorld")
  (Utilities|IsValid _lightreference
    (:Is%20Valid
      (Transformation|AttachActorToActor _lightreference "None" "SnapToTarget" "SnapToTarget" "KeepRelative" true))))

(fn OnIntensityChanged
  (params (NewValue :type Float%20%28single-precision%29))
  (bind _ui_info (Variables|Options|GetUI_Info))
  (bind _color (Utilities|Struct|BreakFButtonInfo _ui_info))
  (bind _secondaryslide (Utilities|Struct|BreakFColorWheelInfo _color))
  (bind _desiredvaluerange (Utilities|Struct|BreakFSlideInfo _secondaryslide))
  (bind (_x _y) (Math|Vector2D|BreakVector2D _desiredvaluerange))
  (bind _aslight (Utilities|Casting|CastToLight (Variables|Options|GetLightReference)))
  (Rendering|Components|Light|SetIntensity (Variables|/Script/Engine.Light|GetLightComponent _aslight) (Math|Float|MapRangeClamped NewValue 0.0 1.0 _x _y)))

(fn OnColorChange
  (bind _aslight (Utilities|Casting|CastToLight (Variables|Options|GetLightReference)))
  (Rendering|Components|Light|SetLightColor (Variables|/Script/Engine.Light|GetLightComponent _aslight) (.DesiredColor (Utilities|Struct|BreakFColorWheelInfo (.Color (Utilities|Struct|BreakFButtonInfo (Variables|Options|GetUI_Info))))) true))

(fn OnUpdateInfo
  (params (NewInfo :type F%20Button%20Info%20Structure))
  (Variables|Options|SetUI_Info NewInfo))