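; Base ArchVis actor for configurable props whose color, material, mesh and decal options can be previewed or recorded in a save table.
; Apply functions use dynamic material instances and propagate changes to RelatedMeshes that share the option type.
; Child actors handle the decal and the edit gizmo, with Moveable forced off except on DynamicActor_BP.
; Touches on main or related meshes notify the character, and custom depth toggles their outline.
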(event OnInputTouchBegin(Mesh)
  (params (FingerIndex :type ETouchIndex%20Enum :default "Touch1") (TouchedComponent :type Primitive%20Component%20Object%20Reference))
  ;[1 1 1] Setup touch event on mesh for mobile or touch screen devices
  (Utilities|IsValid (Variables|Helper|GetCharRef)
    (:Is%20Valid
      (Default|TouchonActor (Variables|Helper|GetCharRef) true))))

(event Custom|RelatedMeshTouch
  (params (FingerIndex :type ETouchIndex%20Enum) (TouchedActor :type Actor%20Object%20Reference))
  ;[1 1 1] Setup touch event on mesh for mobile or touch screen devices
  (Utilities|IsValid (Variables|Helper|GetCharRef)
    (:Is%20Valid
      (Default|TouchonActor (Variables|Helper|GetCharRef) true))))

(event EventBeginPlay
  (bind _mesh (Variables|Components|GetMesh))
  ;[1 1 1] Bind touch event on related meshes
  (for _array_element (Variables|Options|GetRelatedMeshes)
    (EventDispatchers|BindEventtoOnInputTouchBegin (.Mesh (Utilities|Struct|BreakFRelatedMeshOptionInfo _array_element)) (delegate Custom|RelatedMeshTouch)))
  (if (== (Utilities|GetClass self) "/Game/ArchVis/Blueprint/Actor/DynamicActor_BP.DynamicActor_BP_C")
    _
    (else
      (Variables|Options|SetbMoveable false)))
  ;[1 1 1] Save initial location & rotation to add offset later if we need
  (Variables|Helper|SetInitialLocation (Transformation|GetWorldLocation _mesh))
  (Variables|Helper|SetInitialRotation (Transformation|GetWorldRotation _mesh))
  (Transformation|SetWorldRotation (Variables|Default|GetEditComponent) "0, 0, 0" false false))

(fn ConstructionScript
  (bind _decaloptions (Variables|Options|GetDecalOptions))
  (bind _decalsize (Variables|Decal|GetDecalSize))
  (bind _decaloffset (Variables|Decal|GetDecalOffset))
  (bind _item (Utilities|Array|Get(acopy) _decaloptions))
  (bind (_location _rotation) (Math|Transform|BreakTransform _decaloffset))
  (bind _decalmaterialinstance (Utilities|Struct|BreakFDecalOptionInfo _item))
  ;[1 1 1] Initialize UI info for options
  (Variables|UI|SetUI_Color (Utilities|Struct|MakeFButtonInfo "NewEnumerator11" (.displayname (Variables|UI|GetUI_Color)) (.fontsize (Variables|UI|GetUI_Color)) (.textspace (Variables|UI|GetUI_Color)) (.size (Variables|UI|GetUI_Color)) (.normal (Variables|UI|GetUI_Color)) (.hovered (Variables|UI|GetUI_Color)) (.selected (Variables|UI|GetUI_Color)) (.slide (Variables|UI|GetUI_Color)) (.color (Variables|UI|GetUI_Color)) "NewEnumerator7" (.bspacetoenter (Variables|UI|GetUI_Color))))
  (Variables|UI|SetUI_Material (Utilities|Struct|MakeFButtonInfo "NewEnumerator12" (.displayname (Variables|UI|GetUI_Material)) (.fontsize (Variables|UI|GetUI_Material)) (.textspace (Variables|UI|GetUI_Material)) (.size (Variables|UI|GetUI_Material)) (.normal (Variables|UI|GetUI_Material)) (.hovered (Variables|UI|GetUI_Material)) (.selected (Variables|UI|GetUI_Material)) (.slide (Variables|UI|GetUI_Material)) (.color (Variables|UI|GetUI_Material)) "NewEnumerator8" (.bspacetoenter (Variables|UI|GetUI_Material))))
  (Variables|UI|SetUI_Mesh (Utilities|Struct|MakeFButtonInfo "NewEnumerator12" (.displayname (Variables|UI|GetUI_Mesh)) (.fontsize (Variables|UI|GetUI_Mesh)) (.textspace (Variables|UI|GetUI_Mesh)) (.size (Variables|UI|GetUI_Mesh)) (.normal (Variables|UI|GetUI_Mesh)) (.hovered (Variables|UI|GetUI_Mesh)) (.selected (Variables|UI|GetUI_Mesh)) (.slide (Variables|UI|GetUI_Mesh)) (.color (Variables|UI|GetUI_Mesh)) "NewEnumerator9" (.bspacetoenter (Variables|UI|GetUI_Mesh))))
  (Variables|UI|SetUI_Decal (Utilities|Struct|MakeFButtonInfo "NewEnumerator12" (.displayname (Variables|UI|GetUI_Decal)) (.fontsize (Variables|UI|GetUI_Decal)) (.textspace (Variables|UI|GetUI_Decal)) (.size (Variables|UI|GetUI_Decal)) (.normal (Variables|UI|GetUI_Decal)) (.hovered (Variables|UI|GetUI_Decal)) (.selected (Variables|UI|GetUI_Decal)) (.slide (Variables|UI|GetUI_Decal)) (.color (Variables|UI|GetUI_Decal)) "NewEnumerator10" (.bspacetoenter (Variables|UI|GetUI_Decal))))
  ;[1 1 1] Set static mesh to Mesh Component
  (Components|StaticMesh|SetStaticMesh (Variables|Components|GetMesh) (Variables|Options|GetStaticMesh))
  ;[1 1 1] Remove any duplicates from OptionTypes
  (for _array_element (Variables|Options|GetOptionTypes)
    (Utilities|Array|AddUnique (Variables|Options|GetActiveOptions) _array_element))
  ;[1 1 1] To Activate and Unhide decal if decal is one of active options
  (bind _array_element_2 (Utilities|Array|ForEachLoopwithBreak (Variables|Options|GetActiveOptions) :!label _label)
    (:LoopBody
      (if (Utilities|Enum|Equal(Enum) _array_element_2 "NewEnumerator2")
        (bind _asdecal_component_bp (Utilities|Casting|CastToDecalComponent_BP (Variables|/Script/Engine.ChildActorComponent|GetChildActor (Variables|Default|GetDecalComponent_BP))))
        (Rendering|SetVisibility (Variables|/Game/ArchVis/Blueprint/Component/DecalComponent_BP.DecalComponent_BP_C|GetDecalActor _asdecal_component_bp) true true)
        (Development|SetHiddeninGame (Variables|/Game/ArchVis/Blueprint/Component/DecalComponent_BP.DecalComponent_BP_C|GetDecalActor _asdecal_component_bp) false false)
        (goto _label Break)))
    (:Completed
      (Utilities|FlowControl|Sequence
        (:then_0
          ;[1 1 1] Initilize decal
          (bind _asdecal_component_bp_2 (Utilities|Casting|CastToDecalComponent_BP (Variables|/Script/Engine.ChildActorComponent|GetChildActor (Variables|Default|GetDecalComponent_BP))))
          (Transformation|AddLocalOffset (Variables|/Game/ArchVis/Blueprint/Component/DecalComponent_BP.DecalComponent_BP_C|GetDecalActor _asdecal_component_bp_2) _location false false)
          (Transformation|SetWorldRotation (Variables|/Game/ArchVis/Blueprint/Component/DecalComponent_BP.DecalComponent_BP_C|GetDecalActor _asdecal_component_bp_2) _rotation false false)
          (Transformation|SetWorldScale3D (Variables|/Game/ArchVis/Blueprint/Component/DecalComponent_BP.DecalComponent_BP_C|GetDecalActor _asdecal_component_bp_2) (Math|Vector|MakeVector _decalsize _decalsize _decalsize))
          (if (> (Utilities|Array|Length (Variables|Options|GetDecalOptions)) 0)
            (Utilities|IsValid _decalmaterialinstance
              (:Is%20Valid
                (Rendering|Components|Decal|SetDecalMaterial (Variables|/Game/ArchVis/Blueprint/Component/DecalComponent_BP.DecalComponent_BP_C|GetDecalActor _asdecal_component_bp_2) _decalmaterialinstance))
              (:Is%20Not%20Valid
                (Rendering|Components|Decal|SetDecalMaterial (Variables|/Game/ArchVis/Blueprint/Component/DecalComponent_BP.DecalComponent_BP_C|GetDecalActor _asdecal_component_bp_2) "/Game/ArchVis/Material/ArchVis/EpicGamesDecal_MI.EpicGamesDecal_MI" :!label _label_2)))
            (else
              (goto _label_2))))
        (:then_1)))))

(fn ApplyNewColor
  (params (NewInfo :type F%20Color%20Option%20Info%20Structure))
  (LocalVariables|SetColorInfo NewInfo)
  (Helper|CreateMaterialInstace (.MeshIndex (Utilities|Struct|BreakFColorOptionInfo (LocalVariables|GetColorInfo))) "NewEnumerator0")
  (Utilities|FlowControl|Sequence
    (:then_0
      ;[1 1 1] Apply color to main mesh material
      (Utilities|IsValid (Variables|Helper|GetMatInstDynamic)
        (:Is%20Valid
          (Rendering|Material|SetVectorParameterValue (Variables|Helper|GetMatInstDynamic) "Color" (.Color (Utilities|Struct|BreakFColorOptionInfo (LocalVariables|GetColorInfo))) :!class /Script/Engine.MaterialInstanceDynamic)
          (Variables|Helper|SetMatInstDynamic 0))))
    (:then_1
      ;[1 1 1] Apply color to the related meshes material
      (if (> (Utilities|Array|Length (Variables|Options|GetRelatedMeshes)) 0)
        (for _array_element (Variables|Helper|GetRelatedMatInstDynamic)
          (Rendering|Material|SetVectorParameterValue _array_element "Color" (.Color (Utilities|Struct|BreakFColorOptionInfo (LocalVariables|GetColorInfo))) :!class /Script/Engine.MaterialInstanceDynamic))
        (Utilities|Array|Clear (Variables|Helper|GetRelatedMatInstDynamic))))))

(fn CreateMaterialInstace
  (params (NewIndex :type Integer) (NewType :type EOptionTypes%20Enum))
  (bind _mesh (Variables|Components|GetMesh))
  (LocalVariables|SetCurrentType NewType)
  (LocalVariables|SetCurrentIndex NewIndex)
  (Utilities|FlowControl|Sequence
    (:then_0
      ;[1 1 1] Create material instance for desired mesh index and also for related meshes
      (Utilities|IsValid (Variables|Options|GetStaticMesh)
        (:Is%20Valid
          (Utilities|IsValid (Variables|Helper|GetMatInstDynamic)
            (:Is%20Not%20Valid
              (bind _returnvalue (Rendering|Material|CreateDynamicMaterialInstance _mesh (LocalVariables|GetCurrentIndex) (Rendering|Material|GetMaterial _mesh (LocalVariables|GetCurrentIndex)) :!class /Script/Engine.PrimitiveComponent))
              (Variables|Helper|SetMatInstDynamic _returnvalue))))))
    (:then_1
      ;[1 1 1] Creat MaterialInstance for related meshes and add it to array
      (if (> (Utilities|Array|Length (Variables|Options|GetRelatedMeshes)) 0)
        (for _array_element (Variables|Options|GetRelatedMeshes)
          (bind _bnewwants (Helper|CheckSharedOptionTypes (LocalVariables|GetCurrentType) (.OptionTypes (Utilities|Struct|BreakFRelatedMeshOptionInfo _array_element))))
          (LocalVariables|SetbWants _bnewwants)
          ;;[1 1 1] If we need desired option type then create material instance for using in other functions
          (if (LocalVariables|GetbWants)
            (bind _returnvalue_2 (Rendering|Material|CreateDynamicMaterialInstance (Variables|/Script/Engine.StaticMeshActor|GetStaticMeshComponent (.Mesh (Utilities|Struct|BreakFRelatedMeshOptionInfo _array_element))) (select (.bUseSameIndexesAsParent (Utilities|Struct|BreakFRelatedMeshOptionInfo _array_element)) (LocalVariables|GetCurrentIndex) (.MeshIndex (Utilities|Struct|BreakFRelatedMeshOptionInfo _array_element))) (Rendering|Material|GetMaterial (Variables|/Script/Engine.StaticMeshActor|GetStaticMeshComponent (.Mesh (Utilities|Struct|BreakFRelatedMeshOptionInfo _array_element))) (select (.bUseSameIndexesAsParent (Utilities|Struct|BreakFRelatedMeshOptionInfo _array_element)) (LocalVariables|GetCurrentIndex) (.MeshIndex (Utilities|Struct|BreakFRelatedMeshOptionInfo _array_element)))) :!class /Script/Engine.PrimitiveComponent))
            (Utilities|Array|AddUnique (Variables|Helper|GetRelatedMatInstDynamic) _returnvalue_2)))))))

(fn ApplyNewMaterial
  (params (NewInfo :type F%20Material%20Option%20Info%20Structure))
  (LocalVariables|SetMaterialInfo NewInfo)
  (LocalVariables|SetDesiredIndex (.MeshIndex (Utilities|Struct|BreakFMaterialOptionInfo (LocalVariables|GetMaterialInfo))))
  (LocalVariables|SetSourceMaterial (.MaterialInstance (Utilities|Struct|BreakFMaterialOptionInfo (LocalVariables|GetMaterialInfo))))
  ;[1 1 1] Create and apply material on the main mesh
  (bind _returnvalue (Rendering|Material|CreateDynamicMaterialInstance (Variables|Components|GetMesh) (LocalVariables|GetDesiredIndex) (LocalVariables|GetSourceMaterial) :!class /Script/Engine.PrimitiveComponent))
  (Rendering|Material|SetMaterial (Variables|Components|GetMesh) (LocalVariables|GetDesiredIndex) _returnvalue)
  ;[1 1 1] Set material on the related meshes if we shared material option for them
  (if (> (Utilities|Array|Length (Variables|Options|GetRelatedMeshes)) 0)
    (for _array_element (Variables|Options|GetRelatedMeshes)
      (bind _bnewwants (Helper|CheckSharedOptionTypes "NewEnumerator1" (.OptionTypes (Utilities|Struct|BreakFRelatedMeshOptionInfo _array_element))))
      (if _bnewwants
        (bind _returnvalue_2 (Rendering|Material|CreateDynamicMaterialInstance (Variables|/Script/Engine.StaticMeshActor|GetStaticMeshComponent (.Mesh (Utilities|Struct|BreakFRelatedMeshOptionInfo _array_element))) (select (.bUseSameIndexesAsParent (Utilities|Struct|BreakFRelatedMeshOptionInfo _array_element)) (LocalVariables|GetDesiredIndex) (.MeshIndex (Utilities|Struct|BreakFRelatedMeshOptionInfo _array_element))) (LocalVariables|GetSourceMaterial) :!class /Script/Engine.PrimitiveComponent))
        (Rendering|Material|SetMaterial (Variables|/Script/Engine.StaticMeshActor|GetStaticMeshComponent (.Mesh (Utilities|Struct|BreakFRelatedMeshOptionInfo _array_element))) (select (.bUseSameIndexesAsParent (Utilities|Struct|BreakFRelatedMeshOptionInfo _array_element)) (LocalVariables|GetDesiredIndex) (.MeshIndex (Utilities|Struct|BreakFRelatedMeshOptionInfo _array_element))) _returnvalue_2)))))

(fn CheckSharedOptionTypes
  (params (NewDesiredType :type EOptionTypes%20Enum) (NewTypes :type Array%20of%20EOptionTypes%20Enums))
  (LocalVariables|SetCurrentType NewDesiredType)
  ;[1 1 1] Check to see if we want to share desired option type
  (bind _array_element (Utilities|Array|ForEachLoopwithBreak NewTypes :!label _label)
    (:LoopBody
      (bind _output_get (LocalVariables|SetbWants (Utilities|Enum|Equal(Enum) _array_element (LocalVariables|GetCurrentType))))
      (if _output_get
        (goto _label Break)))
    (:Completed
      (return (LocalVariables|GetbWants)))))

(fn ApplyNewMesh
  (params (NewInfo :type F%20Mesh%20Option%20Info%20Structure))
  (bind _initialrotation (Variables|Helper|GetInitialRotation))
  (LocalVariables|SetMeshInfo NewInfo)
  (LocalVariables|SetNewMesh (.Mesh (Utilities|Struct|BreakFMeshOptionInfo (LocalVariables|GetMeshInfo))))
  (LocalVariables|SetNewTransform (.MeshTransform (Utilities|Struct|BreakFMeshOptionInfo (LocalVariables|GetMeshInfo))))
  ;[1 1 1] Set Mesh info on the main mesh, The new static Mesh, Scale, Offset Location & Offset Rotation
  (Components|StaticMesh|SetStaticMesh (Variables|Components|GetMesh) (LocalVariables|GetNewMesh))
  (Transformation|SetWorldScale3D (Variables|Components|GetMesh) (.scale (LocalVariables|GetNewTransform)))
  (Transformation|SetWorldLocation (Variables|Components|GetMesh) (+ (.location (LocalVariables|GetNewTransform)) (Variables|Helper|GetInitialLocation)) false false)
  (Transformation|SetWorldRotation (Variables|Components|GetMesh) (Math|Rotator|MakeRotator (+ (.Roll (Math|Rotator|BreakRotator (.rotation (LocalVariables|GetNewTransform)))) (.roll _initialrotation)) (+ (.Pitch (Math|Rotator|BreakRotator (.rotation (LocalVariables|GetNewTransform)))) (.pitch _initialrotation)) (+ (.Yaw (Math|Rotator|BreakRotator (.rotation (LocalVariables|GetNewTransform)))) (.yaw _initialrotation))) false false)
  ;[1 1 1] Set new mesh on the related mesh actors
  (if (> (Utilities|Array|Length (Variables|Options|GetRelatedMeshes)) 0)
    (for _array_element (Variables|Options|GetRelatedMeshes)
      (bind _bnewwants (Helper|CheckSharedOptionTypes "NewEnumerator3" (.OptionTypes (Utilities|Struct|BreakFRelatedMeshOptionInfo _array_element))))
      (if _bnewwants
        (Components|StaticMesh|SetStaticMesh (Variables|/Script/Engine.StaticMeshActor|GetStaticMeshComponent (.Mesh (Utilities|Struct|BreakFRelatedMeshOptionInfo _array_element))) (LocalVariables|GetNewMesh))))))

(fn ApplyNewDecal
  (params (NewInfo :type F%20Decal%20Option%20Info%20Structure))
  ;[1 1 1] Set the Min/Max decal size and new decal material
  (bind _asdecal_component_bp (Utilities|Casting|CastToDecalComponent_BP (Variables|/Script/Engine.ChildActorComponent|GetChildActor (Variables|Default|GetDecalComponent_BP))))
  (Default|ApplyNewDecal _asdecal_component_bp NewInfo))

(fn ApplyNewColorbyIndex
  (params (NewIndex :type Integer) (bNewPreview :type Boolean))
  (if (and (> NewIndex -1) (< NewIndex (Utilities|Array|Length (Variables|Options|GetColorOptions))))
    (Options|ApplyNewColor (Utilities|Array|Get(acopy) (Variables|Options|GetColorOptions) NewIndex))
    (if (not bNewPreview)
      ;[1 1 1] Update save table
      (Variables|Save|SetSaveTable (Utilities|Struct|MakeSaveTable_BP self NewIndex (.materialindex (Variables|Save|GetSaveTable)) (.meshindex (Variables|Save|GetSaveTable)) (.decalindex (Variables|Save|GetSaveTable)) (Transformation|GetActorTransform))))))

(fn ApplyNewMaterialbyIndex
  (params (NewIndex :type Integer) (bNewPreview :type Boolean))
  (if (and (> NewIndex -1) (< NewIndex (Utilities|Array|Length (Variables|Options|GetMaterialOptions))))
    (Options|ApplyNewMaterial (Utilities|Array|Get(acopy) (Variables|Options|GetMaterialOptions) NewIndex))
    (if (not bNewPreview)
      ;[1 1 1] Update save table
      (Variables|Save|SetSaveTable (Utilities|Struct|MakeSaveTable_BP self (.colorindex (Variables|Save|GetSaveTable)) NewIndex (.meshindex (Variables|Save|GetSaveTable)) (.decalindex (Variables|Save|GetSaveTable)) (Transformation|GetActorTransform))))))

(fn ApplyNewMeshbyIndex
  (params (NewIndex :type Integer) (bNewPreview :type Boolean))
  (if (and (> NewIndex -1) (< NewIndex (Utilities|Array|Length (Variables|Options|GetMeshOptions))))
    (Options|ApplyNewMesh (Utilities|Array|Get(acopy) (Variables|Options|GetMeshOptions) NewIndex))
    (if (not bNewPreview)
      ;[1 1 1] Update save table
      (Variables|Save|SetSaveTable (Utilities|Struct|MakeSaveTable_BP self (.colorindex (Variables|Save|GetSaveTable)) (.materialindex (Variables|Save|GetSaveTable)) NewIndex (.decalindex (Variables|Save|GetSaveTable)) (Transformation|GetActorTransform))))))

(fn ApplyNewDecalbyIndex
  (params (NewIndex :type Integer) (bNewPreview :type Boolean))
  (if (and (> NewIndex -1) (< NewIndex (Utilities|Array|Length (Variables|Options|GetDecalOptions))))
    (Options|ApplyNewDecal (Utilities|Array|Get(acopy) (Variables|Options|GetDecalOptions) NewIndex))
    (if (not bNewPreview)
      ;[1 1 1] Update save table
      (Variables|Save|SetSaveTable (Utilities|Struct|MakeSaveTable_BP self (.colorindex (Variables|Save|GetSaveTable)) (.materialindex (Variables|Save|GetSaveTable)) (.meshindex (Variables|Save|GetSaveTable)) NewIndex (Transformation|GetActorTransform))))))

(fn ToggleEditMode
  (params (bNewEnable :type Boolean) (NewEditType :type EEditTypes%20Enum))
  (LocalVariables|SetEnable bNewEnable)
  (bind _asedit_component_bp (Utilities|Casting|CastToEditComponent_BP (Variables|/Script/Engine.ChildActorComponent|GetChildActor (Variables|Default|GetEditComponent))))
  (Default|ToggleEditGizmo _asedit_component_bp (LocalVariables|GetEnable) NewEditType))

(fn UpdateMeshCollisionResponse
  (params (bNewEnable :type Boolean))
  (bind _returnvalue (select bNewEnable "ECR_Ignore" "ECR_Block"))
  (Collision|SetCollisionResponsetoChannel (Variables|Components|GetMesh) "ECC_Camera" _returnvalue)
  (Collision|SetCollisionResponsetoChannel (Variables|Components|GetMesh) "ECC_Visibility" _returnvalue))

(fn OnMove
  (params (NewXRate :type Float%20%28single-precision%29) (NewYRate :type Float%20%28single-precision%29) (bNewActivateGizmo :type Boolean))
  ;[1 1 1] Call move function on edit component
  (bind _asedit_component_bp (Utilities|Casting|CastToEditComponent_BP (Variables|/Script/Engine.ChildActorComponent|GetChildActor (Variables|Default|GetEditComponent))))
  (Default|OnMove _asedit_component_bp NewXRate NewYRate bNewActivateGizmo))

(fn UpdateGizmoScale
  (params (NewDistance :type Float%20%28single-precision%29))
  ;[1 1 1] Call update gizmo scale on edit component
  (bind _asedit_component_bp (Utilities|Casting|CastToEditComponent_BP (Variables|/Script/Engine.ChildActorComponent|GetChildActor (Variables|Default|GetEditComponent))))
  (Default|UpdateGizmoScale _asedit_component_bp NewDistance))

(fn ToggleMeshRenderDepth
  (params (bNewEnable :type Boolean))
  (bind _output_get (LocalVariables|SetbEnable bNewEnable))
  (Rendering|SetRenderCustomDepth (Variables|Components|GetMesh) _output_get)
  ;[1 1 1] Toggle outline on related meshes
  (for _array_element (Variables|Options|GetRelatedMeshes)
    (Utilities|IsValid (.Mesh (Utilities|Struct|BreakFRelatedMeshOptionInfo _array_element))
      (:Is%20Valid
        (Rendering|SetRenderCustomDepth (Variables|/Script/Engine.StaticMeshActor|GetStaticMeshComponent (.Mesh (Utilities|Struct|BreakFRelatedMeshOptionInfo _array_element))) (LocalVariables|GetbEnable))))))

(fn GetSaveTable
  (bind _savetable (Variables|Save|GetSaveTable))
  (bind (_actor _colorindex _materialindex _meshindex _decalindex _transform _profilename) (Utilities|Struct|BreakSaveTable_BP _savetable))
  (return (Utilities|Struct|MakeSaveTable_BP _actor _colorindex _materialindex _meshindex _decalindex (Transformation|GetActorTransform) _profilename (Transformation|GetWorldTransform (Variables|Default|GetDecalComponent_BP)))))

(fn LoadSaveTable
  (params (NewSaveTable :type Save%20Table%20BP%20Structure))
  (bind (_actor _colorindex _materialindex _meshindex _decalindex _transform _profilename _decaltransform) (Utilities|Struct|BreakSaveTable_BP NewSaveTable))
  (Variables|Save|SetSaveTable (Utilities|Struct|MakeSaveTable_BP self _colorindex _materialindex _meshindex _decalindex _transform _profilename _decaltransform false)))

(fn SetCharRef
  (params (NewChar :type Character%20BP%20Object%20Reference))
  (Variables|Helper|SetCharRef NewChar))