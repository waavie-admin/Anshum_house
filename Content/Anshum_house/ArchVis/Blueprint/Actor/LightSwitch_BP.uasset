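; LightSwitch_BP is a wall light switch actor for an ArchVis scene that turns its linked lights on and off.
; Its collision volume tells Character_BP to show or hide a switch prompt, and touching the base mesh calls ToggleOn.
; ToggleSwitch tilts the switch, then sets each LightsInfo entry's light intensity.
; SetBrightnessOnMesh matches fixture glow to that state through dynamic material instances, created anew on every toggle.
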(event OnComponentBeginOverlap(Collision)
  (params (OverlappedComponent :type Primitive%20Component%20Object%20Reference) (OtherActor :type Actor%20Object%20Reference) (OtherComp :type Primitive%20Component%20Object%20Reference) (OtherBodyIndex :type Integer) (bFromSweep :type Boolean) (SweepResult :type Hit%20Result%20Structure%20%28by%20ref%29))
  ;[1 1 1] Show hide light switch message on character
  (bind _ascharacter_bp (Utilities|Casting|CastToCharacter_BP OtherActor))
  (Default|ToggleLightMessage _ascharacter_bp true self))

(event OnComponentEndOverlap(Collision)
  (params (OverlappedComponent :type Primitive%20Component%20Object%20Reference) (OtherActor :type Actor%20Object%20Reference) (OtherComp :type Primitive%20Component%20Object%20Reference) (OtherBodyIndex :type Integer))
  ;[1 1 1] Show hide light switch message on character
  (bind _ascharacter_bp (Utilities|Casting|CastToCharacter_BP OtherActor))
  (Default|ToggleLightMessage _ascharacter_bp false))

(event OnInputTouchBegin(BaseMesh)
  (params (FingerIndex :type ETouchIndex%20Enum :default "Touch1") (TouchedComponent :type Primitive%20Component%20Object%20Reference))
  ;[1 1 1] Toggle light on/off by touching
  (CallFunction|Toggleon))

(fn ConstructionScript)

(fn ToggleSwitch
  ;[1 1 1] Change rotation on switch
  (Transformation|SetRelativeRotation (Variables|Default|GetSwitch) (select (Variables|Default|GetbOn) "0,0,-5.000000" "0,0,5.000000") false false)
  ;[1 1 1] Set light brightness for all related lights
  (for _array_element (Variables|Default|GetLightsInfo)
    (Utilities|IsValid (.LightRef (Utilities|Struct|BreakFSwitchLightInfo _array_element))
      (:Is%20Valid
        (Rendering|Components|Light|SetIntensity (Variables|/Script/Engine.Light|GetLightComponent (.LightRef (Utilities|Struct|BreakFSwitchLightInfo _array_element))) (select (Variables|Default|GetbOn) (.Intensity (Utilities|Struct|BreakFSwitchLightInfo _array_element)) 0.0)))))
  (CallFunction|SetBrightnessonMesh))

(fn SetBrightnessonMesh
  ;[1 1 1] Set brightness on the mesh of light
  (for _array_element (Variables|Default|GetLightsInfo)
    (Utilities|IsValid (.Mesh (Utilities|Struct|BreakFSwitchLightInfo _array_element))
      (:Is%20Valid
        (bind _returnvalue (Rendering|Material|CreateDynamicMaterialInstance (Variables|/Script/Engine.StaticMeshActor|GetStaticMeshComponent (.Mesh (Utilities|Struct|BreakFSwitchLightInfo _array_element))) (.MeshIndex (Utilities|Struct|BreakFSwitchLightInfo _array_element)) (Rendering|Material|GetMaterial (Variables|/Script/Engine.StaticMeshActor|GetStaticMeshComponent (.Mesh (Utilities|Struct|BreakFSwitchLightInfo _array_element))) (.MeshIndex (Utilities|Struct|BreakFSwitchLightInfo _array_element))) :!class /Script/Engine.PrimitiveComponent))
        (Rendering|Material|SetScalarParameterValue _returnvalue (.MatParamName (Utilities|Struct|BreakFSwitchLightInfo _array_element)) (select (Variables|Default|GetbOn) (.MatBrightness (Utilities|Struct|BreakFSwitchLightInfo _array_element)) 0.0) :!class /Script/Engine.MaterialInstanceDynamic)))))

(fn Toggleon
  ;[1 1 1] Toggle light on or of
  (Variables|Default|SetbOn (not (Variables|Default|GetbOn)))
  (CallFunction|ToggleSwitch))