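; Scale gizmo actor for ArchVis that resizes its grandparent actor along X, Y, Z or all axes.
; Click and touch events on axis handles set the current axis and active state, which can also be set through controller functions.
; OnMove adds frame-time-scaled input rates to the actor's scale, inverting the delta for Z alone.
; UpdateScale resizes the handles by distance, clamped between minimum and maximum scales.
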(event OnClicked(X)
  (params (TouchedComponent :type Primitive%20Component%20Object%20Reference) (ButtonPressed :type Key%20Structure :default "AnyKey"))
  ;[1 1 1] Click/ Touch begin on X axis
  (Variables|Default|SetCurrentAxis "NewEnumerator0")
  (Variables|Default|SetbGizmoActive true))

(event OnInputTouchBegin(X)
  (params (FingerIndex :type ETouchIndex%20Enum :default "Touch1") (TouchedComponent :type Primitive%20Component%20Object%20Reference))
  ;[1 1 1] Click/ Touch begin on X axis
  (Variables|Default|SetCurrentAxis "NewEnumerator0")
  (Variables|Default|SetbGizmoActive true))

(event OnReleased(Y)
  (params (TouchedComponent :type Primitive%20Component%20Object%20Reference) (ButtonReleased :type Key%20Structure :default "AnyKey"))
  ;[1 1 1] Click/ Touch end on Y axis
  (Variables|Default|SetCurrentAxis "NewEnumerator4")
  (Variables|Default|SetbGizmoActive false))

(event OnInputTouchEnd(Y)
  (params (FingerIndex :type ETouchIndex%20Enum :default "Touch1") (TouchedComponent :type Primitive%20Component%20Object%20Reference))
  ;[1 1 1] Click/ Touch end on Y axis
  (Variables|Default|SetCurrentAxis "NewEnumerator4")
  (Variables|Default|SetbGizmoActive false))

(event OnClicked(Y_Box)
  (params (TouchedComponent :type Primitive%20Component%20Object%20Reference) (ButtonPressed :type Key%20Structure :default "AnyKey"))
  ;[1 1 1] Click/ Touch begin on Y axis
  (Variables|Default|SetCurrentAxis "NewEnumerator1")
  (Variables|Default|SetbGizmoActive true))

(event OnInputTouchBegin(Y_Box)
  (params (FingerIndex :type ETouchIndex%20Enum :default "Touch1") (TouchedComponent :type Primitive%20Component%20Object%20Reference))
  ;[1 1 1] Click/ Touch begin on Y axis
  (Variables|Default|SetCurrentAxis "NewEnumerator1")
  (Variables|Default|SetbGizmoActive true))

(event OnReleased(Y_Box)
  (params (TouchedComponent :type Primitive%20Component%20Object%20Reference) (ButtonReleased :type Key%20Structure :default "AnyKey"))
  ;[1 1 1] Click/ Touch end on Y axis
  (Variables|Default|SetCurrentAxis "NewEnumerator4")
  (Variables|Default|SetbGizmoActive false))

(event OnInputTouchEnd(Y_Box)
  (params (FingerIndex :type ETouchIndex%20Enum :default "Touch1") (TouchedComponent :type Primitive%20Component%20Object%20Reference))
  ;[1 1 1] Click/ Touch end on Y axis
  (Variables|Default|SetCurrentAxis "NewEnumerator4")
  (Variables|Default|SetbGizmoActive false))

(event OnClicked(Z)
  (params (TouchedComponent :type Primitive%20Component%20Object%20Reference) (ButtonPressed :type Key%20Structure :default "AnyKey"))
  ;[1 1 1] Click/ Touch begin on Z axis
  (Variables|Default|SetCurrentAxis "NewEnumerator2")
  (Variables|Default|SetbGizmoActive true))

(event OnInputTouchBegin(Z)
  (params (FingerIndex :type ETouchIndex%20Enum :default "Touch1") (TouchedComponent :type Primitive%20Component%20Object%20Reference))
  ;[1 1 1] Click/ Touch begin on Z axis
  (Variables|Default|SetCurrentAxis "NewEnumerator2")
  (Variables|Default|SetbGizmoActive true))

(event OnClicked(Z_Box)
  (params (TouchedComponent :type Primitive%20Component%20Object%20Reference) (ButtonPressed :type Key%20Structure :default "AnyKey"))
  ;[1 1 1] Click/ Touch begin on Z axis
  (Variables|Default|SetCurrentAxis "NewEnumerator2")
  (Variables|Default|SetbGizmoActive true))

(event OnInputTouchBegin(Z_Box)
  (params (FingerIndex :type ETouchIndex%20Enum :default "Touch1") (TouchedComponent :type Primitive%20Component%20Object%20Reference))
  ;[1 1 1] Click/ Touch begin on Z axis
  (Variables|Default|SetCurrentAxis "NewEnumerator2")
  (Variables|Default|SetbGizmoActive true))

(event OnClicked(X_Box)
  (params (TouchedComponent :type Primitive%20Component%20Object%20Reference) (ButtonPressed :type Key%20Structure :default "AnyKey"))
  ;[1 1 1] Click/ Touch begin on X axis
  (Variables|Default|SetCurrentAxis "NewEnumerator0")
  (Variables|Default|SetbGizmoActive true))

(event OnReleased(Z_Box)
  (params (TouchedComponent :type Primitive%20Component%20Object%20Reference) (ButtonReleased :type Key%20Structure :default "AnyKey"))
  ;[1 1 1] Click/ Touch end on Z axis
  (Variables|Default|SetCurrentAxis "NewEnumerator4")
  (Variables|Default|SetbGizmoActive false))

(event OnInputTouchEnd(Z_Box)
  (params (FingerIndex :type ETouchIndex%20Enum :default "Touch1") (TouchedComponent :type Primitive%20Component%20Object%20Reference))
  ;[1 1 1] Click/ Touch end on Z axis
  (Variables|Default|SetCurrentAxis "NewEnumerator4")
  (Variables|Default|SetbGizmoActive false))

(event OnReleased(Z)
  (params (TouchedComponent :type Primitive%20Component%20Object%20Reference) (ButtonReleased :type Key%20Structure :default "AnyKey"))
  ;[1 1 1] Click/ Touch end on Z axis
  (Variables|Default|SetCurrentAxis "NewEnumerator4")
  (Variables|Default|SetbGizmoActive false))

(event OnInputTouchEnd(Z)
  (params (FingerIndex :type ETouchIndex%20Enum :default "Touch1") (TouchedComponent :type Primitive%20Component%20Object%20Reference))
  ;[1 1 1] Click/ Touch end on Z axis
  (Variables|Default|SetCurrentAxis "NewEnumerator4")
  (Variables|Default|SetbGizmoActive false))

(event OnClicked(All)
  (params (TouchedComponent :type Primitive%20Component%20Object%20Reference) (ButtonPressed :type Key%20Structure :default "AnyKey"))
  ;[1 1 1] Click/ Touch begin on all axis
  (Variables|Default|SetCurrentAxis "NewEnumerator3")
  (Variables|Default|SetbGizmoActive true))

(event OnInputTouchBegin(All)
  (params (FingerIndex :type ETouchIndex%20Enum :default "Touch1") (TouchedComponent :type Primitive%20Component%20Object%20Reference))
  ;[1 1 1] Click/ Touch begin on all axis
  (Variables|Default|SetCurrentAxis "NewEnumerator3")
  (Variables|Default|SetbGizmoActive true))

(event OnReleased(All)
  (params (TouchedComponent :type Primitive%20Component%20Object%20Reference) (ButtonReleased :type Key%20Structure :default "AnyKey"))
  ;[1 1 1] Click/ Touch end on all axis
  (Variables|Default|SetCurrentAxis "NewEnumerator4")
  (Variables|Default|SetbGizmoActive false))

(event OnInputTouchEnd(All)
  (params (FingerIndex :type ETouchIndex%20Enum :default "Touch1") (TouchedComponent :type Primitive%20Component%20Object%20Reference))
  ;[1 1 1] Click/ Touch end on all axis
  (Variables|Default|SetCurrentAxis "NewEnumerator4")
  (Variables|Default|SetbGizmoActive false))

(event OnInputTouchBegin(X_Box)
  (params (FingerIndex :type ETouchIndex%20Enum :default "Touch1") (TouchedComponent :type Primitive%20Component%20Object%20Reference))
  ;[1 1 1] Click/ Touch begin on X axis
  (Variables|Default|SetCurrentAxis "NewEnumerator0")
  (Variables|Default|SetbGizmoActive true))

(event OnReleased(X)
  (params (TouchedComponent :type Primitive%20Component%20Object%20Reference) (ButtonReleased :type Key%20Structure :default "AnyKey"))
  ;[1 1 1] Click/ Touch end on X axis
  (Variables|Default|SetCurrentAxis "NewEnumerator4")
  (Variables|Default|SetbGizmoActive false))

(event OnInputTouchEnd(X)
  (params (FingerIndex :type ETouchIndex%20Enum :default "Touch1") (TouchedComponent :type Primitive%20Component%20Object%20Reference))
  ;[1 1 1] Click/ Touch end on X axis
  (Variables|Default|SetCurrentAxis "NewEnumerator4")
  (Variables|Default|SetbGizmoActive false))

(event OnReleased(X_Box)
  (params (TouchedComponent :type Primitive%20Component%20Object%20Reference) (ButtonReleased :type Key%20Structure :default "AnyKey"))
  ;[1 1 1] Click/ Touch end on X axis
  (Variables|Default|SetCurrentAxis "NewEnumerator4")
  (Variables|Default|SetbGizmoActive false))

(event OnInputTouchEnd(X_Box)
  (params (FingerIndex :type ETouchIndex%20Enum :default "Touch1") (TouchedComponent :type Primitive%20Component%20Object%20Reference))
  ;[1 1 1] Click/ Touch end on X axis
  (Variables|Default|SetCurrentAxis "NewEnumerator4")
  (Variables|Default|SetbGizmoActive false))

(event OnClicked(Y)
  (params (TouchedComponent :type Primitive%20Component%20Object%20Reference) (ButtonPressed :type Key%20Structure :default "AnyKey"))
  ;[1 1 1] Click/ Touch begin on Y axis
  (Variables|Default|SetCurrentAxis "NewEnumerator1")
  (Variables|Default|SetbGizmoActive true))

(event OnInputTouchBegin(Y)
  (params (FingerIndex :type ETouchIndex%20Enum :default "Touch1") (TouchedComponent :type Primitive%20Component%20Object%20Reference))
  ;[1 1 1] Click/ Touch begin on Y axis
  (Variables|Default|SetCurrentAxis "NewEnumerator1")
  (Variables|Default|SetbGizmoActive true))

(fn ConstructionScript
  (Transformation|AttachComponentToComponent (Variables|Default|GetX_Box) (Variables|Default|GetX) "Cone_Attachpoint" "SnapToTarget" "SnapToTarget" "KeepWorld" true)
  (Transformation|AttachComponentToComponent (Variables|Default|GetY_Box) (Variables|Default|GetY) "Cone_Attachpoint" "SnapToTarget" "SnapToTarget" "KeepWorld" true)
  (Transformation|AttachComponentToComponent (Variables|Default|GetZ_Box) (Variables|Default|GetZ) "Cone_Attachpoint" "SnapToTarget" "SnapToTarget" "KeepWorld" true))

(fn UpdateScale
  (params (NewDistance :type Float%20%28single-precision%29))
  (bind _maxdistance (Variables|Default|GetMaxDistance))
  (bind _mindistance (Variables|Default|GetMinDistance))
  (bind _minscale (Variables|Default|GetMinScale))
  (bind _maxscale (Variables|Default|GetMaxScale))
  (bind _returnvalue (Math|Float|MapRangeClamped NewDistance _mindistance _maxdistance 0.0 1.0))
  (bind _returnvalue_2 (Math|Float|MapRangeClamped _returnvalue 0.0 1.0 _minscale _maxscale))
  ;[1 1 1] Update gizmo scale depend on distance to player
  (LocalVariables|SetDefaultAllScale "3.000000,3.000000,3.000000")
  (LocalVariables|SetNewCylinderScale (* (Variables|Default|GetDefaultCylinderScale) _returnvalue_2))
  (Utilities|FlowControl|Sequence
    (:then_0
      (Transformation|SetWorldScale3D (Variables|Default|GetX) (LocalVariables|GetNewCylinderScale)))
    (:then_1
      (Transformation|SetWorldScale3D (Variables|Default|GetY) (LocalVariables|GetNewCylinderScale)))
    (:then_2
      (Transformation|SetWorldScale3D (Variables|Default|GetZ) (LocalVariables|GetNewCylinderScale)))
    (:then_3
      (Transformation|SetWorldScale3D (Variables|Default|GetAll) (* (LocalVariables|GetDefaultAllScale) _returnvalue_2)))))

(fn OnMove
  (params (NewXRate :type Float%20%28single-precision%29) (NewYRate :type Float%20%28single-precision%29))
  (bind _returnvalue (Actor|GetParentActor))
  (bind _returnvalue_2 (Utilities|Time|GetWorldDeltaSeconds))
  (bind _movespeed (Variables|Default|GetMoveSpeed))
  (bind _returnvalue_3 (Actor|GetParentActor _returnvalue))
  (bind _returnvalue_4 (* NewXRate _movespeed _returnvalue_2))
  (bind _returnvalue_5 (* NewYRate _movespeed _returnvalue_2))
  (bind _returnvalue_6 (+ _returnvalue_4 _returnvalue_5))
  ;[1 1 1] Calculte scale from current actor scale and new change rate then apply on actor depend on selected axis
  (if (or (Variables|Default|GetbGizmoActive) (Variables|Default|GetbWasController))
    (LocalVariables|SetCurrentActorScale (Transformation|GetActorScale3D _returnvalue_3))
    (Transformation|SetActorScale3D _returnvalue_3 (Utilities|Select :Index (Variables|Default|GetCurrentAxis) :NewEnumerator4 (LocalVariables|GetCurrentActorScale) :NewEnumerator0 (Math|Vector|MakeVector (+ _returnvalue_6 (.x (LocalVariables|GetCurrentActorScale))) (.y (LocalVariables|GetCurrentActorScale)) (.z (LocalVariables|GetCurrentActorScale))) :NewEnumerator1 (Math|Vector|MakeVector (.x (LocalVariables|GetCurrentActorScale)) (+ _returnvalue_6 (.y (LocalVariables|GetCurrentActorScale))) (.z (LocalVariables|GetCurrentActorScale))) :NewEnumerator2 (Math|Vector|MakeVector (.x (LocalVariables|GetCurrentActorScale)) (.y (LocalVariables|GetCurrentActorScale)) (+ (* _returnvalue_6 -1.0) (.z (LocalVariables|GetCurrentActorScale)))) :NewEnumerator3 (Math|Vector|MakeVector (+ _returnvalue_6 (.x (LocalVariables|GetCurrentActorScale))) (+ _returnvalue_6 (.y (LocalVariables|GetCurrentActorScale))) (+ _returnvalue_6 (.z (LocalVariables|GetCurrentActorScale))))))))

(fn ToggleControllerGizmoAxis
  (params (NewAxis :type ETransformAxis%20Enum))
  (Variables|Default|SetCurrentAxis NewAxis))

(fn ActivateGizmo
  (params (bNewEnable :type Boolean))
  (Variables|Default|SetbWasController bNewEnable))