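; Editable decal for the ArchVis scene that can change its material and be manipulated with gizmos.
; On begin play it snaps the child edit component to the decal and zeroes its world rotation.
; It forwards move input, controller axis toggles and cycling through three gizmo types to that child EditComponent_BP.
; Gizmo scale updates from the decal's distance to a supplied location.
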(event EventBeginPlay
  (Transformation|AttachComponentToComponent (Variables|Default|GetEditComponent_BP) (Variables|Default|GetDecalActor) "None" "SnapToTarget" "KeepWorld" "KeepWorld" true)
  (Transformation|SetWorldRotation (Variables|Default|GetEditComponent_BP) "0, 0, 0" false false))

(fn ConstructionScript)

(fn ApplyNewDecal
  (params (NewInfo :type F%20Decal%20Option%20Info%20Structure))
  ;[1 1 1] Set  new decal material
  (Rendering|Components|Decal|SetDecalMaterial (Variables|Default|GetDecalActor) (.DecalMaterialInstance (Utilities|Struct|BreakFDecalOptionInfo NewInfo))))

(fn OnMove
  (params (NewXRate :type Float%20%28single-precision%29) (NewYRate :type Float%20%28single-precision%29) (bNewActivateGizmo :type Boolean))
  ;[1 1 1] Call move function on edit component
  (bind _asedit_component_bp (Utilities|Casting|CastToEditComponent_BP (Variables|/Script/Engine.ChildActorComponent|GetChildActor (Variables|Default|GetEditComponent_BP))))
  (Default|OnMove _asedit_component_bp NewXRate NewYRate bNewActivateGizmo))

(fn ToggleEditMode
  ;[1 1 1] Toggle active gizmo
  (if (== (Variables|Default|GetCurrentGizmoIndex) 2)
    (Variables|Default|SetCurrentGizmoIndex 0)
    (else
      (Variables|Default|SetCurrentGizmoIndex (Math|Integer|Clamp(Integer) (+ (Variables|Default|GetCurrentGizmoIndex) 1) 0 2))))
  (bind _asedit_component_bp (Utilities|Casting|CastToEditComponent_BP (Variables|/Script/Engine.ChildActorComponent|GetChildActor (Variables|Default|GetEditComponent_BP))))
  (Default|ToggleEditGizmo _asedit_component_bp true (Utilities|Array|Get(acopy) (Variables|Default|GetGizmo) (Variables|Default|GetCurrentGizmoIndex))))

(fn UpdateGizmoScale
  (params (NewCurrentLocation :type Vector))
  ;[1 1 1] Update gizmo scale
  (bind _asedit_component_bp (Utilities|Casting|CastToEditComponent_BP (Variables|/Script/Engine.ChildActorComponent|GetChildActor (Variables|Default|GetEditComponent_BP))))
  (Default|UpdateGizmoScale _asedit_component_bp (Math|Vector|VectorLength (- (Transformation|GetWorldLocation (Variables|Default|GetDecalActor)) NewCurrentLocation))))

(fn ToggleAxis
  ;[1 1 1] Toggle axis (X,Y,Z) from controller
  (bind _asedit_component_bp (Utilities|Casting|CastToEditComponent_BP (Variables|/Script/Engine.ChildActorComponent|GetChildActor (Variables|Default|GetEditComponent_BP))))
  (Default|ToggleControllerGizmoAxis _asedit_component_bp))