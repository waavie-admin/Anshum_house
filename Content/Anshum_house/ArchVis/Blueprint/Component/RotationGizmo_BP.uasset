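; Rotation gizmo with Yaw, Pitch and Roll handles that rotates the actor two parent levels above it.
; Clicking or touching a handle sets the active axis, while controllers select it through ToggleControllerGizmoAxis and ActivateGizmo.
; OnMove adds frame-time-scaled input from both move rates to the selected rotation axis.
; While a handle is held, UpdateScale resizes all three handles by clamped player distance.
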(event OnClicked(Yaw)
  (params (TouchedComponent :type Primitive%20Component%20Object%20Reference) (ButtonPressed :type Key%20Structure :default "AnyKey"))
  ;[1 1 1] Click/ Touch begin on Yaw axis
  (Variables|Default|SetCurrentAxis "NewEnumerator2")
  (Variables|Default|SetbGizmoActive true))

(event OnInputTouchBegin(Yaw)
  (params (FingerIndex :type ETouchIndex%20Enum :default "Touch1") (TouchedComponent :type Primitive%20Component%20Object%20Reference))
  ;[1 1 1] Click/ Touch begin on Yaw axis
  (Variables|Default|SetCurrentAxis "NewEnumerator2")
  (Variables|Default|SetbGizmoActive true))

(event OnReleased(Yaw)
  (params (TouchedComponent :type Primitive%20Component%20Object%20Reference) (ButtonReleased :type Key%20Structure :default "AnyKey"))
  ;[1 1 1] Click/ Touch end on Yaw axis
  (Variables|Default|SetCurrentAxis "NewEnumerator4")
  (Variables|Default|SetbGizmoActive false))

(event OnInputTouchEnd(Yaw)
  (params (FingerIndex :type ETouchIndex%20Enum :default "Touch1") (TouchedComponent :type Primitive%20Component%20Object%20Reference))
  ;[1 1 1] Click/ Touch end on Yaw axis
  (Variables|Default|SetCurrentAxis "NewEnumerator4")
  (Variables|Default|SetbGizmoActive false))

(event OnClicked(Pitch)
  (params (TouchedComponent :type Primitive%20Component%20Object%20Reference) (ButtonPressed :type Key%20Structure :default "AnyKey"))
  ;[1 1 1] Click/ Touch Begin on Pitch axis
  (Variables|Default|SetCurrentAxis "NewEnumerator1")
  (Variables|Default|SetbGizmoActive true))

(event OnInputTouchBegin(Pitch)
  (params (FingerIndex :type ETouchIndex%20Enum :default "Touch1") (TouchedComponent :type Primitive%20Component%20Object%20Reference))
  ;[1 1 1] Click/ Touch Begin on Pitch axis
  (Variables|Default|SetCurrentAxis "NewEnumerator1")
  (Variables|Default|SetbGizmoActive true))

(event OnInputTouchEnd(Pitch)
  (params (FingerIndex :type ETouchIndex%20Enum :default "Touch1") (TouchedComponent :type Primitive%20Component%20Object%20Reference))
  ;[1 1 1] Click/ Touch end on Pitch axis
  (Variables|Default|SetCurrentAxis "NewEnumerator4")
  (Variables|Default|SetbGizmoActive false))

(event OnReleased(Pitch)
  (params (TouchedComponent :type Primitive%20Component%20Object%20Reference) (ButtonReleased :type Key%20Structure :default "AnyKey"))
  ;[1 1 1] Click/ Touch end on Pitch axis
  (Variables|Default|SetCurrentAxis "NewEnumerator4")
  (Variables|Default|SetbGizmoActive false))

(event OnClicked(Roll)
  (params (TouchedComponent :type Primitive%20Component%20Object%20Reference) (ButtonPressed :type Key%20Structure :default "AnyKey"))
  ;[1 1 1] Click/ Touch Begin on Roll axis
  (Variables|Default|SetCurrentAxis "NewEnumerator0")
  (Variables|Default|SetbGizmoActive true))

(event OnInputTouchBegin(Roll)
  (params (FingerIndex :type ETouchIndex%20Enum :default "Touch1") (TouchedComponent :type Primitive%20Component%20Object%20Reference))
  ;[1 1 1] Click/ Touch Begin on Roll axis
  (Variables|Default|SetCurrentAxis "NewEnumerator0")
  (Variables|Default|SetbGizmoActive true))

(event OnReleased(Roll)
  (params (TouchedComponent :type Primitive%20Component%20Object%20Reference) (ButtonReleased :type Key%20Structure :default "AnyKey"))
  ;[1 1 1] Click/ Touch Begin on Roll axis
  (Variables|Default|SetCurrentAxis "NewEnumerator4")
  (Variables|Default|SetbGizmoActive false))

(event OnInputTouchEnd(Roll)
  (params (FingerIndex :type ETouchIndex%20Enum :default "Touch1") (TouchedComponent :type Primitive%20Component%20Object%20Reference))
  ;[1 1 1] Click/ Touch Begin on Roll axis
  (Variables|Default|SetCurrentAxis "NewEnumerator4")
  (Variables|Default|SetbGizmoActive false))

(fn ConstructionScript)

(fn OnMove
  (params (NewXRate :type Float%20%28single-precision%29) (NewYRate :type Float%20%28single-precision%29))
  (bind _returnvalue (Actor|GetParentActor))
  (bind _returnvalue_2 (Utilities|Time|GetWorldDeltaSeconds))
  (bind _movespeed (Variables|Default|GetMoveSpeed))
  (bind _returnvalue_3 (Actor|GetParentActor _returnvalue))
  ;[1 1 1] Calculate new actor rotation base on current rotation and axis move rate
  (if (or (Variables|Default|GetbGizmoActive) (Variables|Default|GetbWasController))
    (LocalVariables|SetRate (+ (* NewXRate _movespeed _returnvalue_2) (* NewYRate _movespeed _returnvalue_2)))
    (bind _output_get (LocalVariables|SetCurrentActorRotation (Transformation|GetActorRotation _returnvalue_3)))
    (Transformation|SetActorRotation _returnvalue_3 (Utilities|Select :Index (Variables|Default|GetCurrentAxis) :NewEnumerator4 _output_get :NewEnumerator0 (Math|Rotator|MakeRotator (+ (.roll (LocalVariables|GetCurrentActorRotation)) (LocalVariables|GetRate)) (.pitch (LocalVariables|GetCurrentActorRotation)) (.yaw (LocalVariables|GetCurrentActorRotation))) :NewEnumerator1 (Math|Rotator|MakeRotator (.roll (LocalVariables|GetCurrentActorRotation)) (+ (.pitch (LocalVariables|GetCurrentActorRotation)) (LocalVariables|GetRate)) (.yaw (LocalVariables|GetCurrentActorRotation))) :NewEnumerator2 (Math|Rotator|MakeRotator (.roll (LocalVariables|GetCurrentActorRotation)) (.pitch (LocalVariables|GetCurrentActorRotation)) (+ (LocalVariables|GetRate) (.yaw (LocalVariables|GetCurrentActorRotation)))) :NewEnumerator3 ""))))

(fn UpdateScale
  (params (NewDistance :type Float%20%28single-precision%29))
  ;[1 1 1] Update gizmo scale depend on distance to player
  (if (Variables|Default|GetbGizmoActive)
    (LocalVariables|SetNewPlaneScale (* (Variables|Default|GetDefaultPlaneScale) (Math|Float|MapRangeClamped (Math|Float|MapRangeClamped NewDistance (Variables|Default|GetMinDistance) (Variables|Default|GetMaxDistance) 0.0 1.0) 0.0 1.0 (Variables|Default|GetMinScale) (Variables|Default|GetMaxScale))))
    (Utilities|FlowControl|Sequence
      (:then_0
        (Transformation|SetWorldScale3D (Variables|Default|GetYaw) (LocalVariables|GetNewPlaneScale)))
      (:then_1
        (Transformation|SetWorldScale3D (Variables|Default|GetPitch) (LocalVariables|GetNewPlaneScale)))
      (:then_2
        (Transformation|SetWorldScale3D (Variables|Default|GetRoll) (LocalVariables|GetNewPlaneScale))))))

(fn ToggleControllerGizmoAxis
  (params (NewAxis :type ETransformAxis%20Enum))
  (Variables|Default|SetCurrentAxis NewAxis))

(fn ActivateGizmo
  (params (bNewEnable :type Boolean))
  (Variables|Default|SetbWasController bNewEnable))