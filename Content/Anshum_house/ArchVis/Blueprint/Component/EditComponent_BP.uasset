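; EditComponent_BP manages location, rotation and scale transform gizmos for editing in an ArchVis project.
; Each gizmo is a child actor, hidden with collision off at BeginPlay, and ToggleEditGizmo shows or hides the one matching the edit type.
; Move rates with the active controller and distance-based scale updates are forwarded to the current gizmo.
; Controller axis toggling cycles an index through EditAxis, with one extra step for scale.
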(event EventBeginPlay
  (bind _locationgizmo_bp (Variables|Default|GetLocationGizmo_BP))
  (bind _rotationgizmo_bp (Variables|Default|GetRotationGizmo_BP))
  (bind _scalegizmo_bp (Variables|Default|GetScaleGizmo_BP))
  ;[1 1 1] Set hidden for all gizmo
  (Rendering|SetVisibility _locationgizmo_bp false true)
  (Collision|SetActorEnableCollision (Variables|/Script/Engine.ChildActorComponent|GetChildActor _locationgizmo_bp) false)
  (Rendering|SetVisibility _rotationgizmo_bp false true)
  (Collision|SetActorEnableCollision (Variables|/Script/Engine.ChildActorComponent|GetChildActor _rotationgizmo_bp) false)
  (Rendering|SetVisibility _scalegizmo_bp false true)
  (Collision|SetActorEnableCollision (Variables|/Script/Engine.ChildActorComponent|GetChildActor _scalegizmo_bp) false))

(fn ConstructionScript)

(fn ToggleEditGizmo
  (params (NewEnable :type Boolean) (NewEditType :type EEditTypes%20Enum))
  (bind _locationgizmo_bp (Variables|Default|GetLocationGizmo_BP))
  (bind _rotationgizmo_bp (Variables|Default|GetRotationGizmo_BP))
  (bind _locationgizmo_bp_2 (Variables|Default|GetLocationGizmo_BP))
  (bind _rotationgizmo_bp_2 (Variables|Default|GetRotationGizmo_BP))
  (bind _scalegizmo_bp (Variables|Default|GetScaleGizmo_BP))
  (bind _scalegizmo_bp_2 (Variables|Default|GetScaleGizmo_BP))
  (LocalVariables|SetEditType NewEditType)
  (if NewEnable
    ;[1 1 1] Set Collision and Visibility on for desired component
    (bind _output_get (Variables|Default|SetCurrentType (LocalVariables|GetEditType)))
    (switch Utilities|FlowControl|Switch|SwitchonEEditTypes _output_get
      (:NewEnumerator0
        (Rendering|SetVisibility _locationgizmo_bp true true)
        (Collision|SetActorEnableCollision (Variables|/Script/Engine.ChildActorComponent|GetChildActor _locationgizmo_bp) true)
        (Rendering|SetVisibility (Variables|Default|GetRotationGizmo_BP) false true)
        (Rendering|SetVisibility (Variables|Default|GetScaleGizmo_BP) false true))
      (:NewEnumerator1
        (Rendering|SetVisibility (Variables|Default|GetLocationGizmo_BP) false true)
        (Rendering|SetVisibility _rotationgizmo_bp true true)
        (Collision|SetActorEnableCollision (Variables|/Script/Engine.ChildActorComponent|GetChildActor _rotationgizmo_bp) true)
        (Rendering|SetVisibility (Variables|Default|GetScaleGizmo_BP) false true))
      (:NewEnumerator2
        (Rendering|SetVisibility (Variables|Default|GetLocationGizmo_BP) false true)
        (Rendering|SetVisibility (Variables|Default|GetRotationGizmo_BP) false true)
        (Rendering|SetVisibility _scalegizmo_bp_2 true true)
        (Collision|SetActorEnableCollision (Variables|/Script/Engine.ChildActorComponent|GetChildActor _scalegizmo_bp_2) true)))
    (else
      ;[1 1 1] Set Collision and Visibility off for desired component
      (switch Utilities|FlowControl|Switch|SwitchonEEditTypes (LocalVariables|GetEditType)
        (:NewEnumerator0
          (Rendering|SetVisibility _locationgizmo_bp_2 false true)
          (Collision|SetActorEnableCollision (Variables|/Script/Engine.ChildActorComponent|GetChildActor _locationgizmo_bp_2) false))
        (:NewEnumerator1
          (Rendering|SetVisibility _rotationgizmo_bp_2 false true)
          (Collision|SetActorEnableCollision (Variables|/Script/Engine.ChildActorComponent|GetChildActor _rotationgizmo_bp_2) false))
        (:NewEnumerator2
          (Rendering|SetVisibility _scalegizmo_bp false true)
          (Collision|SetActorEnableCollision (Variables|/Script/Engine.ChildActorComponent|GetChildActor _scalegizmo_bp) false))))))

(fn OnMove
  (params (NewXRate :type Float%20%28single-precision%29) (NewYRate :type Float%20%28single-precision%29) (bNewController :type Boolean))
  (LocalVariables|SetActiveController bNewController)
  ;[1 1 1] Send move rate to current active gizmo
  (LocalVariables|SetXRate NewXRate)
  (LocalVariables|SetYRate NewYRate)
  (switch Utilities|FlowControl|Switch|SwitchonEEditTypes (Variables|Default|GetCurrentType)
    (:NewEnumerator0
      (bind _aslocation_gizmo_bp (Utilities|Casting|CastToLocationGizmo_BP (Variables|/Script/Engine.ChildActorComponent|GetChildActor (Variables|Default|GetLocationGizmo_BP))))
      (Default|OnMove _aslocation_gizmo_bp (LocalVariables|GetXRate) (LocalVariables|GetYRate))
      (Default|ActivateGizmo _aslocation_gizmo_bp (LocalVariables|GetActiveController)))
    (:NewEnumerator1
      (bind _asrotation_gizmo_bp (Utilities|Casting|CastToRotationGizmo_BP (Variables|/Script/Engine.ChildActorComponent|GetChildActor (Variables|Default|GetRotationGizmo_BP))))
      (Default|OnMove _asrotation_gizmo_bp (LocalVariables|GetXRate) (LocalVariables|GetYRate))
      (Default|ActivateGizmo _asrotation_gizmo_bp (LocalVariables|GetActiveController)))
    (:NewEnumerator2
      (bind _asscale_gizmo_bp (Utilities|Casting|CastToScaleGizmo_BP (Variables|/Script/Engine.ChildActorComponent|GetChildActor (Variables|Default|GetScaleGizmo_BP))))
      (Default|OnMove _asscale_gizmo_bp (LocalVariables|GetXRate) (LocalVariables|GetYRate))
      (Default|ActivateGizmo _asscale_gizmo_bp (LocalVariables|GetActiveController)))))

(fn UpdateGizmoScale
  (params (NewDistance :type Float%20%28single-precision%29))
  ;[1 1 1] Update gizmo scale
  (LocalVariables|SetDistance NewDistance)
  (switch Utilities|FlowControl|Switch|SwitchonEEditTypes (Variables|Default|GetCurrentType)
    (:NewEnumerator0
      (bind _aslocation_gizmo_bp (Utilities|Casting|CastToLocationGizmo_BP (Variables|/Script/Engine.ChildActorComponent|GetChildActor (Variables|Default|GetLocationGizmo_BP))))
      (Default|UpdateScale _aslocation_gizmo_bp (LocalVariables|GetDistance)))
    (:NewEnumerator1
      (bind _asrotation_gizmo_bp (Utilities|Casting|CastToRotationGizmo_BP (Variables|/Script/Engine.ChildActorComponent|GetChildActor (Variables|Default|GetRotationGizmo_BP))))
      (Default|UpdateScale _asrotation_gizmo_bp (LocalVariables|GetDistance)))
    (:NewEnumerator2
      (bind _asscale_gizmo_bp (Utilities|Casting|CastToScaleGizmo_BP (Variables|/Script/Engine.ChildActorComponent|GetChildActor (Variables|Default|GetScaleGizmo_BP))))
      (Default|UpdateScale _asscale_gizmo_bp (LocalVariables|GetDistance)))))

(fn ToggleControllerGizmoAxis
  ;[1 1 1] Toggle axis for gizmo
  (if (Utilities|Select :Index (Variables|Default|GetCurrentType) :NewEnumerator0 (== (Variables|Default|GetCurrentGizmoIndex) 2) :NewEnumerator1 (== (Variables|Default|GetCurrentGizmoIndex) 2) :NewEnumerator2 (== (Variables|Default|GetCurrentGizmoIndex) 3))
    (Variables|Default|SetCurrentGizmoIndex 0)
    (else
      (Variables|Default|SetCurrentGizmoIndex (Utilities|Select :Index (Variables|Default|GetCurrentType) :NewEnumerator0 (Math|Integer|Clamp(Integer) (+ (Variables|Default|GetCurrentGizmoIndex) 1) 0 2) :NewEnumerator1 (Math|Integer|Clamp(Integer) (+ (Variables|Default|GetCurrentGizmoIndex) 1) 0 2) :NewEnumerator2 (Math|Integer|Clamp(Integer) (+ (Variables|Default|GetCurrentGizmoIndex) 1) 0 3)))))
  (switch Utilities|FlowControl|Switch|SwitchonEEditTypes (Variables|Default|GetCurrentType)
    (:NewEnumerator0
      (bind _aslocation_gizmo_bp (Utilities|Casting|CastToLocationGizmo_BP (Variables|/Script/Engine.ChildActorComponent|GetChildActor (Variables|Default|GetLocationGizmo_BP))))
      (Default|ToggleControllerGizmoAxis _aslocation_gizmo_bp (Utilities|Array|Get(acopy) (Variables|Default|GetEditAxis) (Variables|Default|GetCurrentGizmoIndex))))
    (:NewEnumerator1
      (bind _asrotation_gizmo_bp (Utilities|Casting|CastToRotationGizmo_BP (Variables|/Script/Engine.ChildActorComponent|GetChildActor (Variables|Default|GetRotationGizmo_BP))))
      (Default|ToggleControllerGizmoAxis _asrotation_gizmo_bp (Utilities|Array|Get(acopy) (Variables|Default|GetEditAxis) (Variables|Default|GetCurrentGizmoIndex))))
    (:NewEnumerator2
      (bind _asscale_gizmo_bp (Utilities|Casting|CastToScaleGizmo_BP (Variables|/Script/Engine.ChildActorComponent|GetChildActor (Variables|Default|GetScaleGizmo_BP))))
      (Default|ToggleControllerGizmoAxis _asscale_gizmo_bp (Utilities|Array|Get(acopy) (Variables|Default|GetEditAxis) (Variables|Default|GetCurrentGizmoIndex))))))