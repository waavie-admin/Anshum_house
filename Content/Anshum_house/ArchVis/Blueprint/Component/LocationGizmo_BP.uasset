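; Translation gizmo that moves the actor two parent levels above it along a world X, Y or Z axis.
; Click or touch on an axis shaft or its socket-attached cone sets the active axis until release, while separate functions let controller input pick the axis and enable movement.
; OnMove sums both input rates into a frame-time-scaled offset, negated for Z.
; UpdateScale resizes the shafts by clamped distance.
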(event OnClicked(X)
  (params (TouchedComponent :type Primitive%20Component%20Object%20Reference) (ButtonPressed :type Key%20Structure :default "AnyKey"))
  ;[1 1 1] Click/ Touch begin on X axis
  (Variables|Default|SetCurrentAxis "NewEnumerator0")
  (Variables|Default|SetbGizmoActive true))

(event OnClicked(X_Cone)
  (params (TouchedComponent :type Primitive%20Component%20Object%20Reference) (ButtonPressed :type Key%20Structure :default "AnyKey"))
  ;[1 1 1] Click/ Touch begin on X axis
  (Variables|Default|SetCurrentAxis "NewEnumerator0")
  (Variables|Default|SetbGizmoActive true))

(event OnClicked(Z_Cone)
  (params (TouchedComponent :type Primitive%20Component%20Object%20Reference) (ButtonPressed :type Key%20Structure :default "AnyKey"))
  ;[1 1 1] Click/ Touch begin on Z axis
  (Variables|Default|SetCurrentAxis "NewEnumerator2")
  (Variables|Default|SetbGizmoActive true))

(event OnInputTouchBegin(Z_Cone)
  (params (FingerIndex :type ETouchIndex%20Enum :default "Touch1") (TouchedComponent :type Primitive%20Component%20Object%20Reference))
  ;[1 1 1] Click/ Touch begin on Z axis
  (Variables|Default|SetCurrentAxis "NewEnumerator2")
  (Variables|Default|SetbGizmoActive true))

(event OnInputTouchBegin(X)
  (params (FingerIndex :type ETouchIndex%20Enum :default "Touch1") (TouchedComponent :type Primitive%20Component%20Object%20Reference))
  ;[1 1 1] Click/ Touch begin on X axis
  (Variables|Default|SetCurrentAxis "NewEnumerator0")
  (Variables|Default|SetbGizmoActive true))

(event OnInputTouchBegin(X_Cone)
  (params (FingerIndex :type ETouchIndex%20Enum :default "Touch1") (TouchedComponent :type Primitive%20Component%20Object%20Reference))
  ;[1 1 1] Click/ Touch begin on X axis
  (Variables|Default|SetCurrentAxis "NewEnumerator0")
  (Variables|Default|SetbGizmoActive true))

(event OnReleased(X)
  (params (TouchedComponent :type Primitive%20Component%20Object%20Reference) (ButtonReleased :type Key%20Structure :default "AnyKey"))
  ;[1 1 1] Click/ Touch end on X axis
  (Variables|Default|SetCurrentAxis "NewEnumerator4")
  (Variables|Default|SetbGizmoActive false))

(event OnReleased(X_Cone)
  (params (TouchedComponent :type Primitive%20Component%20Object%20Reference) (ButtonReleased :type Key%20Structure :default "AnyKey"))
  ;[1 1 1] Click/ Touch end on X axis
  (Variables|Default|SetCurrentAxis "NewEnumerator4")
  (Variables|Default|SetbGizmoActive false))

(event OnClicked(Y)
  (params (TouchedComponent :type Primitive%20Component%20Object%20Reference) (ButtonPressed :type Key%20Structure :default "AnyKey"))
  ;[1 1 1] Click/ Touch begin on Y axis
  (Variables|Default|SetCurrentAxis "NewEnumerator1")
  (Variables|Default|SetbGizmoActive true))

(event OnInputTouchEnd(X)
  (params (FingerIndex :type ETouchIndex%20Enum :default "Touch1") (TouchedComponent :type Primitive%20Component%20Object%20Reference))
  ;[1 1 1] Click/ Touch end on X axis
  (Variables|Default|SetCurrentAxis "NewEnumerator4")
  (Variables|Default|SetbGizmoActive false))

(event OnInputTouchEnd(X_Cone)
  (params (FingerIndex :type ETouchIndex%20Enum :default "Touch1") (TouchedComponent :type Primitive%20Component%20Object%20Reference))
  ;[1 1 1] Click/ Touch end on X axis
  (Variables|Default|SetCurrentAxis "NewEnumerator4")
  (Variables|Default|SetbGizmoActive false))

(event OnReleased(Y)
  (params (TouchedComponent :type Primitive%20Component%20Object%20Reference) (ButtonReleased :type Key%20Structure :default "AnyKey"))
  ;[1 1 1] Click/ Touch end on Y axis
  (Variables|Default|SetCurrentAxis "NewEnumerator4")
  (Variables|Default|SetbGizmoActive false))

(event OnInputTouchBegin(Y)
  (params (FingerIndex :type ETouchIndex%20Enum :default "Touch1") (TouchedComponent :type Primitive%20Component%20Object%20Reference))
  ;[1 1 1] Click/ Touch begin on Y axis
  (Variables|Default|SetCurrentAxis "NewEnumerator1")
  (Variables|Default|SetbGizmoActive true))

(event OnReleased(Y_Cone)
  (params (TouchedComponent :type Primitive%20Component%20Object%20Reference) (ButtonReleased :type Key%20Structure :default "AnyKey"))
  ;[1 1 1] Click/ Touch end on Y axis
  (Variables|Default|SetCurrentAxis "NewEnumerator4")
  (Variables|Default|SetbGizmoActive false))

(event OnInputTouchEnd(Y)
  (params (FingerIndex :type ETouchIndex%20Enum :default "Touch1") (TouchedComponent :type Primitive%20Component%20Object%20Reference))
  ;[1 1 1] Click/ Touch end on Y axis
  (Variables|Default|SetCurrentAxis "NewEnumerator4")
  (Variables|Default|SetbGizmoActive false))

(event OnInputTouchEnd(Y_Cone)
  (params (FingerIndex :type ETouchIndex%20Enum :default "Touch1") (TouchedComponent :type Primitive%20Component%20Object%20Reference))
  ;[1 1 1] Click/ Touch end on Y axis
  (Variables|Default|SetCurrentAxis "NewEnumerator4")
  (Variables|Default|SetbGizmoActive false))

(event OnReleased(Z)
  (params (TouchedComponent :type Primitive%20Component%20Object%20Reference) (ButtonReleased :type Key%20Structure :default "AnyKey"))
  ;[1 1 1] Click/ Touch end on Z axis
  (Variables|Default|SetCurrentAxis "NewEnumerator4")
  (Variables|Default|SetbGizmoActive false))

(event OnClicked(Y_Cone)
  (params (TouchedComponent :type Primitive%20Component%20Object%20Reference) (ButtonPressed :type Key%20Structure :default "AnyKey"))
  ;[1 1 1] Click/ Touch begin on Y axis
  (Variables|Default|SetCurrentAxis "NewEnumerator1")
  (Variables|Default|SetbGizmoActive true))

(event OnReleased(Z_Cone)
  (params (TouchedComponent :type Primitive%20Component%20Object%20Reference) (ButtonReleased :type Key%20Structure :default "AnyKey"))
  ;[1 1 1] Click/ Touch end on Z axis
  (Variables|Default|SetCurrentAxis "NewEnumerator4")
  (Variables|Default|SetbGizmoActive false))

(event OnInputTouchEnd(Z)
  (params (FingerIndex :type ETouchIndex%20Enum :default "Touch1") (TouchedComponent :type Primitive%20Component%20Object%20Reference))
  ;[1 1 1] Click/ Touch end on Z axis
  (Variables|Default|SetCurrentAxis "NewEnumerator4")
  (Variables|Default|SetbGizmoActive false))

(event OnInputTouchEnd(Z_Cone)
  (params (FingerIndex :type ETouchIndex%20Enum :default "Touch1") (TouchedComponent :type Primitive%20Component%20Object%20Reference))
  ;[1 1 1] Click/ Touch end on Z axis
  (Variables|Default|SetCurrentAxis "NewEnumerator4")
  (Variables|Default|SetbGizmoActive false))

(event OnInputTouchBegin(Y_Cone)
  (params (FingerIndex :type ETouchIndex%20Enum :default "Touch1") (TouchedComponent :type Primitive%20Component%20Object%20Reference))
  ;[1 1 1] Click/ Touch begin on Y axis
  (Variables|Default|SetCurrentAxis "NewEnumerator1")
  (Variables|Default|SetbGizmoActive true))

(event OnClicked(Z)
  (params (TouchedComponent :type Primitive%20Component%20Object%20Reference) (ButtonPressed :type Key%20Structure :default "AnyKey"))
  ;[1 1 1] Click/ Touch begin on Z axis
  (Variables|Default|SetCurrentAxis "NewEnumerator2")
  (Variables|Default|SetbGizmoActive true))

(event OnInputTouchBegin(Z)
  (params (FingerIndex :type ETouchIndex%20Enum :default "Touch1") (TouchedComponent :type Primitive%20Component%20Object%20Reference))
  ;[1 1 1] Click/ Touch begin on Z axis
  (Variables|Default|SetCurrentAxis "NewEnumerator2")
  (Variables|Default|SetbGizmoActive true))

(fn ConstructionScript
  (Transformation|AttachComponentToComponent (Variables|Default|GetX_Cone) (Variables|Default|GetX) "Cone_Attachpoint" "SnapToTarget" "SnapToTarget" "KeepWorld" true)
  (Transformation|AttachComponentToComponent (Variables|Default|GetY_Cone) (Variables|Default|GetY) "Cone_Attachpoint" "SnapToTarget" "SnapToTarget" "KeepWorld" true)
  (Transformation|AttachComponentToComponent (Variables|Default|GetZ_Cone) (Variables|Default|GetZ) "Cone_Attachpoint" "SnapToTarget" "SnapToTarget" "KeepWorld" true))

(fn UpdateScale
  (params (NewDistance :type Float%20%28single-precision%29))
  ;[1 1 1] Update gizmo scale depend on distance to player
  (LocalVariables|SetNewCylinderScale (* (Variables|Default|GetDefaultCylinderScale) (Math|Float|MapRangeClamped (Math|Float|MapRangeClamped NewDistance (Variables|Default|GetMinDistance) (Variables|Default|GetMaxDistance) 0.0 1.0) 0.0 1.0 (Variables|Default|GetMinScale) (Variables|Default|GetMaxScale))))
  (Utilities|FlowControl|Sequence
    (:then_0
      (Transformation|SetWorldScale3D (Variables|Default|GetX) (LocalVariables|GetNewCylinderScale)))
    (:then_1
      (Transformation|SetWorldScale3D (Variables|Default|GetY) (LocalVariables|GetNewCylinderScale)))
    (:then_2
      (Transformation|SetWorldScale3D (Variables|Default|GetZ) (LocalVariables|GetNewCylinderScale)))))

(fn OnMove
  (params (NewXRate :type Float%20%28single-precision%29) (NewYRate :type Float%20%28single-precision%29))
  (bind _returnvalue (Utilities|Time|GetWorldDeltaSeconds))
  (bind _movespeed (Variables|Default|GetMoveSpeed))
  (bind _returnvalue_2 (* NewXRate _movespeed _returnvalue))
  (bind _returnvalue_3 (* NewYRate _movespeed _returnvalue))
  (bind _returnvalue_4 (+ _returnvalue_2 _returnvalue_3))
  ;[1 1 1] Add world offset to selected actor
  (if (or (Variables|Default|GetbGizmoActive) (Variables|Default|GetbWasController))
    (Transformation|AddActorWorldOffset (Actor|GetParentActor (Actor|GetParentActor)) (Utilities|Select :Index (Variables|Default|GetCurrentAxis) :NewEnumerator4 "" :NewEnumerator0 (Math|Vector|MakeVector _returnvalue_4 0.0 0.0) :NewEnumerator1 (Math|Vector|MakeVector 0.0 _returnvalue_4 0.0) :NewEnumerator2 (Math|Vector|MakeVector 0.0 0.0 (* _returnvalue_4 -1.0)) :NewEnumerator3 ""))))

(fn ToggleControllerGizmoAxis
  (params (NewAxis :type ETransformAxis%20Enum))
  (Variables|Default|SetCurrentAxis NewAxis))

(fn ActivateGizmo
  (params (bNewEnable :type Boolean))
  (Variables|Default|SetbWasController bNewEnable))